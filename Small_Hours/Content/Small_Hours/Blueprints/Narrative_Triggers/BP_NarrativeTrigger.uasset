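; BP_NarrativeTrigger is a box trigger that plays a one-time narrative voice line with a subtitle when the player enters during a specific act.
; On overlap it compares the game instance's CurrentAct to TargetAct, and only a match uses up the DoOnce, plays NarrativeVO and shows NarrativeText.
; Each trigger creates its own WBP_NarrativeUI at BeginPlay, starts it hidden, and hides the subtitle when the audio finishes.
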(event `self.Box.OnComponentBeginOverlap`
  (params (OverlappedComponent :type "PrimitiveComponent Object Reference") (OtherActor :type "Actor Object Reference") (OtherComp :type "PrimitiveComponent Object Reference") (OtherBodyIndex :type Integer) (bFromSweep :type Boolean) (SweepResult :type "HitResult Structure (by ref)"))
  (if (== OtherActor (`GameplayStatics.GetPlayerCharacter` 0))
    (bind _asgi_my_game (cast `/Game/Small_Hours/Blueprints/GI_MyGame` (`GameplayStatics.GetGameInstance`)))
    (if (== (`/Game/Small_Hours/Blueprints/GI_MyGame.CurrentAct` _asgi_my_game) (`self.TargetAct`))
      (`/Engine/EditorBlueprintResources/StandardMacros.DoOnce` false
        (:`Completed`
          (`AudioComponent.SetSound` (`self.Audio`) (`self.NarrativeVO`))
          (`AudioComponent.Play` (`self.Audio`) 0.0)
          (`/Game/Small_Hours/UI/WBP_NarrativeUI.ShowSubtitle` (`self.ActiveUI`) (`self.NarrativeText`)))))))

(event `OnAudioFinished_Event`
  (`/Game/Small_Hours/UI/WBP_NarrativeUI.HideSubtitle` (`self.ActiveUI`) :!label _label))

(event `self.ReceiveBeginPlay`
  (bind _returnvalue (`|CreateWidget` "/Game/Small_Hours/UI/WBP_NarrativeUI.WBP_NarrativeUI_C"))
  (bind _output_get (set `self.ActiveUI` _returnvalue))
  (`UserWidget.AddToViewport` _output_get 0)
  (`Widget.SetVisibility` (`/Game/Small_Hours/UI/WBP_NarrativeUI.SubtitleText` (`self.ActiveUI`)) "Hidden")
  (add `AudioComponent.OnAudioFinished` (`self.Audio`) (delegate `OnAudioFinished_Event`))
  (goto _label))

(fn `UserConstructionScript`)