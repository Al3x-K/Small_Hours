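; BP_GameManager runs the transition between acts in Small Hours through its StartActTransition event.
; It disables input, fades to black, increments CurrentAct on GI_MyGame and moves the player to a PlayerStart without loading a level.
; It then shows the WBP_ActTransition widget with music.
; Fixed delays time the sequence, which ends by removing the widget, fading back in and restoring input.
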(event `StartActTransition`
  (bind _returnvalue (`GameplayStatics.GetPlayerController` 0))
  (bind _returnvalue_2 (`GameplayStatics.GetPlayerCameraManager` 0))
  (`self.DisableInput` _returnvalue null)
  (`PlayerCameraManager.StartCameraFade` :`self` _returnvalue_2 :`ToAlpha` 1.0 :`Duration` 1.0 :`bHoldWhenFinished` true)
  (`KismetSystemLibrary.Delay` 1.1)
  (bind _asgi_my_game (cast `/Game/Small_Hours/Blueprints/GI_MyGame` (`GameplayStatics.GetGameInstance`)))
  (set `/Game/Small_Hours/Blueprints/GI_MyGame.CurrentAct` (+ (`/Game/Small_Hours/Blueprints/GI_MyGame.CurrentAct` _asgi_my_game) 1) _asgi_my_game)
  (bind _returnvalue_3 (`GameplayStatics.GetActorOfClass` "/Script/Engine.PlayerStart"))
  (`self.K2_SetActorLocation` (`GameplayStatics.GetPlayerCharacter` 0) (`self.K2_GetActorLocation` _returnvalue_3) false false)
  (bind _returnvalue_4 (`|CreateWidget` "/Game/Small_Hours/UI/WBP_ActTransition.WBP_ActTransition_C"))
  (`UserWidget.AddToViewport` _returnvalue_4 0)
  (`GameplayStatics.PlaySound2D` "/Game/Small_Hours/Audio/Music/MUS_Act_Transition.MUS_Act_Transition" 1.0 1.0 0.0 null null)
  (`KismetSystemLibrary.Delay` 7.2)
  (`Widget.RemoveFromParent` _returnvalue_4)
  (`PlayerCameraManager.StartCameraFade` :`self` _returnvalue_2 :`FromAlpha` 1.0 :`Duration` 1.0)
  (`self.EnableInput` _returnvalue null))

(fn `UserConstructionScript`)