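; A destructible clutter object that the player can clean up during its target act.
; While the game instance's current act matches, overlapping the interaction range shows a widget to the player, and leaving hides it.
; CleanUp repeats the act check, spawns a Niagara break effect, plays a sound at world origin, tells BP_GameManager to update the clutter value, then destroys the actor.
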(event `self.InteractionRange.OnComponentBeginOverlap`
  (params (OverlappedComponent :type "PrimitiveComponent Object Reference") (OtherActor :type "Actor Object Reference") (OtherComp :type "PrimitiveComponent Object Reference") (OtherBodyIndex :type Integer) (bFromSweep :type Boolean) (SweepResult :type "HitResult Structure (by ref)"))
  (bind _asgi_my_game (cast `/Game/Small_Hours/Blueprints/GI_MyGame` (`GameplayStatics.GetGameInstance`)))
  (if (== (`/Game/Small_Hours/Blueprints/GI_MyGame.CurrentAct` _asgi_my_game) (`self.TargetAct`))
    (if (== OtherActor (`GameplayStatics.GetPlayerCharacter` 0))
      (`SceneComponent.SetVisibility` (`self.Widget`) true false))))

(event `self.InteractionRange.OnComponentEndOverlap`
  (params (OverlappedComponent :type "PrimitiveComponent Object Reference") (OtherActor :type "Actor Object Reference") (OtherComp :type "PrimitiveComponent Object Reference") (OtherBodyIndex :type Integer))
  (if (== OtherActor (`GameplayStatics.GetPlayerCharacter` 0))
    (`SceneComponent.SetVisibility` (`self.Widget`) false false)))

(event `/Game/Small_Hours/Blueprints/BPI_Clutter.CleanUp`
  (bind _asgi_my_game (cast `/Game/Small_Hours/Blueprints/GI_MyGame` (`GameplayStatics.GetGameInstance`)))
  (if (== (`/Game/Small_Hours/Blueprints/GI_MyGame.CurrentAct` _asgi_my_game) (`self.TargetAct`))
    (`NiagaraFunctionLibrary.SpawnSystemAtLocation` "/Game/Small_Hours/NS_ClutterBreak.NS_ClutterBreak" (`self.K2_GetActorLocation`) (`self.K2_GetActorRotation`))
    (`GameplayStatics.PlaySoundAtLocation` (`self.CleanUpSound`) (0.0 0.0 0.0) (struct) 1.0 1.0 0.0 null null null null)
    (bind _returnvalue (`GameplayStatics.GetActorOfClass` "/Game/Small_Hours/Blueprints/BP_GameManager.BP_GameManager_C"))
    (`/Game/Small_Hours/Blueprints/BP_GameManager.UpdateClutterValue` _returnvalue)
    (`self.K2_DestroyActor`)))

(fn `UserConstructionScript`)