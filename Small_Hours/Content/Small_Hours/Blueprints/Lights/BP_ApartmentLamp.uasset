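; BP_ApartmentLamp is an apartment lamp whose spotlight switches on or off according to the current act.
; The UpdateLampForAct event turns the light off in act 1 and sets it to BaseIntensity in act 2.
; In act 3, only instances with the HeroLight actor tag stay lit, while all others go dark.
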(event `UpdateLampForAct`
  (params (CurrentAct :type Integer))
  (switch `int` CurrentAct
    (:`1`
      (`LightComponent.SetIntensity` (`self.SpotLight`) 0.0))
    (:`2`
      (`LightComponent.SetIntensity` (`self.SpotLight`) (`self.BaseIntensity`)))
    (:`3`
      (if (`self.ActorHasTag` "HeroLight")
        (`LightComponent.SetIntensity` (`self.SpotLight`) (`self.BaseIntensity`))
        (else
          (`LightComponent.SetIntensity` (`self.SpotLight`) 0.0))))))

(fn `UserConstructionScript`)