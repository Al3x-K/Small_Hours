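; Kitchen lamp actor for the apartment that switches its seven spot lights on or off according to the current act.
; UpdateLampForAct sets every spot light to zero intensity in acts one and three.
; In act two, only lamps with the HeroLight actor tag light up at BaseIntensity, while untagged lamps stay dark.
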(event `UpdateLampForAct`
  (params (CurrentAct :type Integer))
  (switch `int` CurrentAct
    (:`1`
      (for _array_element (`|MakeArray` (`self.SpotLight`) (`self.SpotLight1`) (`self.SpotLight2`) (`self.SpotLight3`) (`self.SpotLight4`) (`self.SpotLight5`) (`self.SpotLight6`))
        (`LightComponent.SetIntensity` _array_element 0.0)))
    (:`2`
      (if (`self.ActorHasTag` "HeroLight")
        (for _array_element_2 (`|MakeArray` (`self.SpotLight`) (`self.SpotLight1`) (`self.SpotLight2`) (`self.SpotLight3`) (`self.SpotLight4`) (`self.SpotLight5`) (`self.SpotLight6`))
          (`LightComponent.SetIntensity` _array_element_2 (`self.BaseIntensity`)))
        (else
          (for _array_element_3 (`|MakeArray` (`self.SpotLight`) (`self.SpotLight1`) (`self.SpotLight2`) (`self.SpotLight3`) (`self.SpotLight4`) (`self.SpotLight5`) (`self.SpotLight6`))
            (`LightComponent.SetIntensity` _array_element_3 0.0)))))
    (:`3`
      (for _array_element_4 (`|MakeArray` (`self.SpotLight`) (`self.SpotLight1`) (`self.SpotLight2`) (`self.SpotLight3`) (`self.SpotLight4`) (`self.SpotLight5`) (`self.SpotLight6`))
        (`LightComponent.SetIntensity` _array_element_4 0.0)))))

(fn `UserConstructionScript`)