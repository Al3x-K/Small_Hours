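; Base Blueprint for inspectable objects that shows an interact prompt when the first-person player enters its sphere.
; The prompt requires the game instance's current act to match TargetAct and the object to be unused.
; RefreshPromptVisibility creates the UI_Interact widget, plays its pop-up, applies an outline overlay material and enables CanPressE.
; Leaving the sphere only hides the widget, and GetInspectMesh is an empty stub.
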(event `self.Sphere.OnComponentBeginOverlap`
  (params (OverlappedComponent :type "PrimitiveComponent Object Reference") (OtherActor :type "Actor Object Reference") (OtherComp :type "PrimitiveComponent Object Reference") (OtherBodyIndex :type Integer) (bFromSweep :type Boolean) (SweepResult :type "HitResult Structure (by ref)"))
  (bind _bhasbeenused (`self.bHasBeenUsed`))
  (cast `/Game/Small_Hours/Blueprints/BP_FirstPersonCharacter` OtherActor)
  (bind _asgi_my_game (cast `/Game/Small_Hours/Blueprints/GI_MyGame` (`GameplayStatics.GetGameInstance`)))
  (if (and (== (`/Game/Small_Hours/Blueprints/GI_MyGame.CurrentAct` _asgi_my_game) (`self.TargetAct`)) (== _bhasbeenused false))
    (`self.RefreshPromptVisibility`)
    (else
      (`SceneComponent.SetHiddenInGame` (`self.Widget`) true false)
      (`KismetSystemLibrary.PrintString` (`KismetStringLibrary.Conv_BoolToString` _bhasbeenused)))))

(event `self.Sphere.OnComponentEndOverlap`
  (params (OverlappedComponent :type "PrimitiveComponent Object Reference") (OtherActor :type "Actor Object Reference") (OtherComp :type "PrimitiveComponent Object Reference") (OtherBodyIndex :type Integer))
  (cast `/Game/Small_Hours/Blueprints/BP_FirstPersonCharacter` OtherActor)
  (`SceneComponent.SetHiddenInGame` (`self.Widget`) true false)
  (`KismetSystemLibrary.PrintString` "Player Left - Forcing Hide"))

(fn `GetInspectMesh`
  (returns (TargetObject :type "StaticMesh Object Reference"))
  (return null))

(fn `RefreshPromptVisibility`
  (bind _widget (`self.Widget`))
  (bind _asgi_my_game (cast `/Game/Small_Hours/Blueprints/GI_MyGame` (`GameplayStatics.GetGameInstance`))
    (:`then`
      (if (and (== (`/Game/Small_Hours/Blueprints/GI_MyGame.CurrentAct` _asgi_my_game) (`self.TargetAct`)) (not (`self.bHasBeenUsed`)))
        (if (`self.HintVisible`)
          (`SceneComponent.SetHiddenInGame` (`self.Widget`) true false)
          (`KismetSystemLibrary.PrintString` "UI Hidden: Act is [CurrentAct] but need [TargetAct] OR Used is [bHasBeenUsed]")
          (else
            (bind _returnvalue (`|CreateWidget` "/Game/Small_Hours/UI/UI_Interact.UI_Interact_C"))
            (bind _output_get (set `self.InteractionWidget` _returnvalue))
            (`WidgetComponent.SetWidget` _widget _output_get)
            (`SceneComponent.SetHiddenInGame` _widget false false)
            (bind _interactionwidget (`self.InteractionWidget`)
              (:`then`
                (if (not (`self.HintVisible`))
                  (`UserWidget.PlayAnimation` _interactionwidget (`/Game/Small_Hours/UI/UI_Interact.PopUp` _interactionwidget) 0.0 1 "Forward" 1.5 false)
                  (set `self.HintVisible` true)
                  (`MeshComponent.SetOverlayMaterial` (`self.StaticMesh`) "/Game/Small_Hours/Materials/M_Outline.M_Outline")
                  (set `self.CanPressE` true)
                  (`KismetSystemLibrary.PrintString` "UI Shown: Conditions Met")
                  (set `self.CanInteract` false)
                  (set `self.HintVisible` false)))
              (:`else`))))))
    (:`CastFailed`
      (`KismetSystemLibrary.PrintString` "cast failed"))))

(fn `UserConstructionScript`)